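; GameResponseManager is an actor that sends a command response through the GameManagerInstance game instance according to which level is running.
; On BeginPlay it compares the current level name with the game instance's GameLevel and OutroLevel.
; The game level triggers a start command response and the outro level an end command response, while any other level only prints that none was sent.
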(event `self.ReceiveBeginPlay`
  (bind _asgame_manager_instance (cast `/Game/GunnerSquad/Blueprints/GameManagerInstance` (`GameplayStatics.GetGameInstance`)))
  (bind _returnvalue (`GameplayStatics.GetCurrentLevelName` true))
  (if (`KismetStringLibrary.EqualEqual_StrStr` _returnvalue (`KismetStringLibrary.Conv_NameToString` (`/Game/GunnerSquad/Blueprints/GameManagerInstance.GameLevel` _asgame_manager_instance)))
    (`WePlayVR_GameInstance.SendStartCommandResponse` _asgame_manager_instance)
    (elif (`KismetStringLibrary.EqualEqual_StrStr` _returnvalue (`KismetStringLibrary.Conv_NameToString` (`/Game/GunnerSquad/Blueprints/GameManagerInstance.OutroLevel` _asgame_manager_instance)))
      (`WePlayVR_GameInstance.SendEndCommandResponse` _asgame_manager_instance)
      (else
        (`KismetSystemLibrary.PrintString` "No Response Sent")))))

(fn `UserConstructionScript`)