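; GunnerSquad game manager Blueprint that advances the game from intro level to game level to outro level through streaming.
; Two ChangeLevel_0 input handlers, labelled Start and End command flows, check the current level name against IntroLevel or GameLevel.
; On a match, each blocking-loads the next stream level as visible, then unloads the previous one, printing debug messages.
; The End key only prints a debug string.
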(event `Key|End`
  (params (Key :type "Key Structure"))
  (:`Pressed`
    (`KismetSystemLibrary.PrintString` "FINISH HIM")))

(event `InputAction|ChangeLevel_0`
  (params (Key :type "Key Structure"))
  ;[1 1 1] Start Command Flow
  (:`Pressed`
    (`KismetSystemLibrary.PrintString` "Change Level: START RECEIVED")
    (bind _returnvalue (`GameplayStatics.GetCurrentLevelName` true))
    (if (`KismetStringLibrary.EqualEqual_StrStr` _returnvalue (`KismetStringLibrary.Conv_NameToString` (`self.IntroLevel`)))
      (bind _output_get (set `self.StreamLevelName` (`self.GameLevel`)))
      (`GameplayStatics.LoadStreamLevel` _output_get true true)
      (bind _output_get_2 (set `self.UnloadLevelName` (`self.IntroLevel`)))
      (`GameplayStatics.UnloadStreamLevel` _output_get_2 true)
      (`KismetSystemLibrary.PrintString` "Level Change Complete"))))

(event `InputAction|ChangeLevel_0`
  (params (Key :type "Key Structure"))
  ;[1 1 1] End Command Flow
  (:`Pressed`
    (`KismetSystemLibrary.PrintString` "Change Level: STOP RECIEVED")
    (bind _returnvalue (`GameplayStatics.GetCurrentLevelName` true))
    (if (`KismetStringLibrary.EqualEqual_StrStr` _returnvalue (`KismetStringLibrary.Conv_NameToString` (`self.GameLevel`)))
      (bind _output_get (set `self.StreamLevelName` (`self.OutroLevel`)))
      (`GameplayStatics.LoadStreamLevel` _output_get true true)
      (bind _output_get_2 (set `self.UnloadLevelName` (`self.GameLevel`)))
      (`GameplayStatics.UnloadStreamLevel` _output_get_2 true)
      (`KismetSystemLibrary.PrintString` "Level Change Complete"))))

(fn `UserConstructionScript`)