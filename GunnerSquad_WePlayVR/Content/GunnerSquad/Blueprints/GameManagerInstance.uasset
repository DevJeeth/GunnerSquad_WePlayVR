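; GameManagerInstance handles level progression for GunnerSquad, moving the game from intro to gameplay to outro in response to start and end commands.
; The start-command event opens the game level only when the intro level is current.
; The end-command event opens the outro level only when the game level is current.
; Both compare the current level name against stored level names and print debug strings when loading.
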(event `self.OnStartCommandReceived`
  (bind _gamelevel (`self.GameLevel`))
  ;[1 1 1] Start command Received
  (bind _returnvalue (`GameplayStatics.GetCurrentLevelName` true))
  (`KismetSystemLibrary.PrintString` _returnvalue)
  (if (`KismetStringLibrary.EqualEqual_StrStr` _returnvalue (`KismetStringLibrary.Conv_NameToString` (`self.IntroLevel`)))
    (`KismetSystemLibrary.PrintString` (`KismetStringLibrary.Concat_StrStr` "Loading: " (`KismetStringLibrary.Conv_NameToString` _gamelevel)))
    (bind _output_get (set `self.StreamLevelName` _gamelevel))
    (`GameplayStatics.OpenLevel` _output_get)))

(event `self.OnEndCommandReceived`
  (bind _outrolevel (`self.OutroLevel`))
  ;[1 1 1] End Command Received
  (bind _returnvalue (`GameplayStatics.GetCurrentLevelName` true))
  (if (`KismetStringLibrary.EqualEqual_StrStr` _returnvalue (`KismetStringLibrary.Conv_NameToString` (`self.GameLevel`)))
    (`KismetSystemLibrary.PrintString` (`KismetStringLibrary.Concat_StrStr` "Loading: " (`KismetStringLibrary.Conv_NameToString` _outrolevel)))
    (bind _output_get (set `self.StreamLevelName` _outrolevel))
    (`GameplayStatics.OpenLevel` _output_get)))