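; Game manager input Blueprint that moves GunnerSquad between its intro, game and outro levels on start and end commands.
; The StartCommand action opens the game level only from the intro level, and EndCommand opens the outro only from the game level.
; Each checks the current level name against level name variables, stores the target in StreamLevelName and opens it by name.
; Debug prints trace the transitions, and the End key prints a test message.
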(event `Key|End`
  (params (Key :type "Key Structure"))
  (:`Pressed`
    (`KismetSystemLibrary.PrintString` "Testing Input Key")))

(event `self.ReceiveBeginPlay`
  ;[1 1 1] Start Command Flow
)

(event `InputAction|StartCommand`
  (params (Key :type "Key Structure"))
  (bind _gamelevel (`self.GameLevel`))
  ;[1 1 1] Start Command Flow
  (:`Pressed`
    (`KismetSystemLibrary.PrintString` "Change Level: START RECEIVED")
    (bind _returnvalue (`GameplayStatics.GetCurrentLevelName` true))
    (`KismetSystemLibrary.PrintString` _returnvalue)
    (if (`KismetStringLibrary.EqualEqual_StrStr` _returnvalue (`KismetStringLibrary.Conv_NameToString` (`self.IntroLevel`)))
      (`KismetSystemLibrary.PrintString` (`KismetStringLibrary.Concat_StrStr` "Loading: " (`KismetStringLibrary.Conv_NameToString` _gamelevel)))
      (bind _output_get (set `self.StreamLevelName` _gamelevel))
      (`GameplayStatics.OpenLevel` _output_get))))

(event `InputAction|EndCommand`
  (params (Key :type "Key Structure"))
  (bind _outrolevel (`self.OutroLevel`))
  ;[1 1 1] End Command Flow
  (:`Pressed`
    (`KismetSystemLibrary.PrintString` "Change Level: STOP RECIEVED")
    (bind _returnvalue (`GameplayStatics.GetCurrentLevelName` true))
    (if (`KismetStringLibrary.EqualEqual_StrStr` _returnvalue (`KismetStringLibrary.Conv_NameToString` (`self.GameLevel`)))
      (`KismetSystemLibrary.PrintString` (`KismetStringLibrary.Concat_StrStr` "Loading: " (`KismetStringLibrary.Conv_NameToString` _outrolevel)))
      (bind _output_get (set `self.StreamLevelName` _outrolevel))
      (`GameplayStatics.OpenLevel` _output_get))))

(fn `UserConstructionScript`)